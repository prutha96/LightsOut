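; BP_Door is a key-locked door that either swings open or loads another level.
; On overlap, it searches the FirstPersonCharacter's OwnedKeys for its required type, removes the match and destroys the character's KeyVar actor.
; Transition doors save the remaining keys to TestGameInstance before opening the named level; others disable collision and rotate via a timeline.
; The construction script colors the frame to match the required key.
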(event OnComponentBeginOverlap(Overlap)
  (params (OverlappedComponent :type Primitive%20Component%20Object%20Reference) (OtherActor :type Actor%20Object%20Reference) (OtherComp :type Primitive%20Component%20Object%20Reference) (OtherBodyIndex :type Integer) (bFromSweep :type Boolean) (SweepResult :type Hit%20Result%20Structure%20%28by%20ref%29))
  (bind _asfirst_person_character (Utilities|Casting|CastToFirstPersonCharacter OtherActor))
  (for (_array_element _array_index) (Variables|/Game/FirstPersonBP/Blueprints/FirstPersonCharacter.FirstPersonCharacter_C|GetOwnedKeys _asfirst_person_character)
    (if (Utilities|Enum|Equal(Enum) _array_element (Variables|Default|GetRequiredKeyType))
      (Utilities|FlowControl|Sequence
        (:then_0
          (Utilities|Array|RemoveIndex (Variables|/Game/FirstPersonBP/Blueprints/FirstPersonCharacter.FirstPersonCharacter_C|GetOwnedKeys _asfirst_person_character) _array_index)
          (if (Variables|Default|GetLevelTransition)
            (bind _astest_game_instance (Utilities|Casting|CastToTestGameInstance (Game|GetGameInstance)))
            (Variables|/Game/TestGameInstance.TestGameInstance_C|SetPlayerKeys _astest_game_instance (Variables|/Game/FirstPersonBP/Blueprints/FirstPersonCharacter.FirstPersonCharacter_C|GetOwnedKeys _asfirst_person_character))
            (Game|OpenLevel(byName) (Variables|Default|GetLevelName))
            (else
              (Collision|SetCollisionEnabled (Variables|Default|GetDoor) "NoCollision")
              (bind _rotz (Timeline|DoorMovement PlayFromStart)
                (:Update
                  (Transformation|SetRelativeRotation (Variables|Default|GetDoor) (Math|Rotator|MakeRotator 0.0 0.0 _rotz) false false))))))
        (:then_1
          (Actor|DestroyActor (Variables|/Game/FirstPersonBP/Blueprints/FirstPersonCharacter.FirstPersonCharacter_C|GetkeyVar _asfirst_person_character)))))))

(fn ConstructionScript
  (Rendering|Material|SetMaterial (Variables|Default|GetFrame) 0 (Utilities|Select :Index (Variables|Default|GetRequiredKeyType) :NewEnumerator0 "/Game/Materials/M_Key.M_Key" :NewEnumerator1 "/Game/Materials/M_RedKey.M_RedKey" :NewEnumerator2 "/Game/Materials/M_GreenKey.M_GreenKey" :NewEnumerator3 "/Game/Materials/M_BlueKey.M_BlueKey")))