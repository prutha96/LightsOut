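; BP_Trigger is a trigger volume that shows a moving SampleFigureBP when the first-person character enters its Box.
; The overlap spawns the figure at a stored location and rotation, then plays a timeline that lerps it from StartPos to EndPos without sweeping.
; When the timeline finishes, it destroys both the figure and the trigger itself.
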(event OnComponentBeginOverlap(Box)
  (params (OverlappedComponent :type Primitive%20Component%20Object%20Reference) (OtherActor :type Actor%20Object%20Reference) (OtherComp :type Primitive%20Component%20Object%20Reference) (OtherBodyIndex :type Integer) (bFromSweep :type Boolean) (SweepResult :type Hit%20Result%20Structure%20%28by%20ref%29))
  (Utilities|Casting|CastToFirstPersonCharacter OtherActor)
  (bind _returnvalue (Game|SpawnActorfromClass "/Game/HorrorEngine/Meshes/SampleFigureBP.SampleFigureBP_C" (Math|Transform|MakeTransform (Variables|Default|GetlocationVar) (Variables|Default|GetrotationVar) "1,1.000000,1") "Undefined" 0 0))
  (bind _alpha (Timeline|Timeline_0 Play)
    (:Update
      (Transformation|SetActorLocation _returnvalue (Math|Vector|Lerp(Vector) (Variables|Default|GetstartPos) (Variables|Default|GetendPos) _alpha) false false))
    (:Finished
      (Actor|DestroyActor _returnvalue)
      (Actor|DestroyActor))))

(event EventBeginPlay)

(event Collision|EventActorBeginOverlap
  (params (OtherActor :type Actor%20Object%20Reference)))

(event EventTick
  (params (DeltaSeconds :type Float%20%28single-precision%29)))

(fn ConstructionScript)