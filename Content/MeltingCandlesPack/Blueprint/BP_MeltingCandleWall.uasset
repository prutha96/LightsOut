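; Melting wall candle, a child candle Blueprint with a selectable or randomized mesh whose flames descend as it melts.
; Construction adds a flame particle, smoke mesh and optional light child actor at wick sockets, storing start/end locations from socket pairs.
; A timeline scaled by MeltTime drives the material's "Anim" parameter and lerps flame positions, optionally destroying the actor when finished.
; MeltPoint also previews the melt state during construction.
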(event Custom|StartMelting
  ;[1 1 1] begin play setup melting time
  (|CallParentFunction)
  (Components|Timeline|SetPlayRate (Variables|Default|GetTimeline_Melting) (/ 1.0 (Variables|Melting|GetMeltTime)))
  (if (Variables|Default|GetCandleFlameOn)
    ;[1 1 1] Start candle flame and melting
    (Components|Timeline|SetNewTime (Variables|Default|GetTimeline_Melting) (Variables|Melting|GetMeltPoint))
    ;[1 1 1] Handles melting animation, light and particle position
    (bind _lerp (Timeline|Timeline_Melting Play)
      (:Update
        (Variables|Melting|SetMeltPoint _lerp)
        (Rendering|Material|SetScalarParameterValue (Variables|Default|GetCandleMaterial) "Anim" (Variables|Melting|GetMeltPoint) :!class /Script/Engine.MaterialInstanceDynamic)
        (if (== (Utilities|Array|Length (Variables|Default|GetFlames)) 1)
          (CallFunction|UpdateFlameLoc 0 (Variables|Melting|GetMeltPoint))
          (else
            (for (_ _array_index) (Variables|Default|GetFlames)
              (CallFunction|UpdateFlameLoc _array_index (Variables|Melting|GetMeltPoint))))))
      (:Finished
        (if (Variables|Melting|GetOffAfterMelt)
          (CallFunction|CandleOff true true)
          (Actor|DestroyActor))))))

(event EventAddCandleEffects
  ;[1 1 1] Add smoke mesh, particles and lights to selected mesh sockets. Construction script use only
  (CallFunction|SetupDynamicEffects))

(event EventSetupCandleMesh
  (bind _enablecandleindexes (Variables|Default|GetEnableCandleIndexes))
  ;[1 1 1] Setup mesh from index and state. Construction script use only
  (if (Variables|Default|GetRandomCandleMesh)
    (bind _keys (Utilities|Map|Keys (Variables|Default|GetEnableIndexInRandom)))
    (for _array_element _keys
      (if (.Value (Utilities|Map|Find (Variables|Default|GetEnableIndexInRandom) _array_element))
        (Utilities|Array|Add (Variables|Default|GetEnableCandleIndexes) _array_element)))
    (Variables|Default|SetCandleMeshIndex (Utilities|Array|Get(acopy) _enablecandleindexes (Math|Random|RandomIntegerinRange 1 (Utilities|Array|LastIndex _enablecandleindexes)))))
  (Components|StaticMesh|SetStaticMesh (Variables|Default|GetSM_Candle) (Utilities|Select :Index (Variables|Default|GetCandleMeshIndex) :Option%200 "/Game/MeltingCandlesPack/AnimatedCandles/1/SM_Candle_Anim_1.SM_Candle_Anim_1" :Option%201 "/Game/MeltingCandlesPack/AnimatedCandles/1/SM_Candle_Anim_1.SM_Candle_Anim_1" :Option%202 "/Game/MeltingCandlesPack/AnimatedCandles/2/SM_Candle_Anim_2.SM_Candle_Anim_2" :Option%203 "/Game/MeltingCandlesPack/AnimatedCandles/3/SM_Candle_Anim_3.SM_Candle_Anim_3" :Option%204 "/Game/MeltingCandlesPack/AnimatedCandles/4/SM_Candle_Anim_4.SM_Candle_Anim_4" :Option%205 "/Game/MeltingCandlesPack/AnimatedCandles/5/SM_Candle_Anim_5.SM_Candle_Anim_5" :Option%206 "/Game/MeltingCandlesPack/AnimatedCandles/6/SM_Candle_Anim_6.SM_Candle_Anim_6" :Option%207 "/Game/MeltingCandlesPack/AnimatedCandles/7/SM_Candle_Anim_7.SM_Candle_Anim_7" :Option%208 "/Game/MeltingCandlesPack/AnimatedCandles/8/SM_Candle_Anim_8.SM_Candle_Anim_8" :Option%209 "/Game/MeltingCandlesPack/AnimatedCandles/9/SM_Candle_Anim_9.SM_Candle_Anim_9" :Option%2010 "/Game/MeltingCandlesPack/AnimatedCandles/10/SM_Candle_Anim_10.SM_Candle_Anim_10" :Option%2011 "/Game/MeltingCandlesPack/AnimatedCandles/11/SM_Candle_Anim_11.SM_Candle_Anim_11" :Option%2012 "/Game/MeltingCandlesPack/AnimatedCandles/12/SM_Candle_Anim_12.SM_Candle_Anim_12" :Option%2013 "/Game/MeltingCandlesPack/AnimatedCandles/13/SM_Candle_Anim_13.SM_Candle_Anim_13" :Option%2014 "/Game/MeltingCandlesPack/AnimatedCandles/14/SM_Candle_Anim_14.SM_Candle_Anim_14")))

(event EventCandleOff
  (params (Cooling :type Boolean) (Smoke :type Boolean))
  ;[1 1 1] stop candle melting and putting candle off
  (|CallParentFunction Cooling Smoke)
  ;[1 1 1] Handles melting animation, light and particle position
  (bind _lerp (Timeline|Timeline_Melting Stop)
    (:Update
      (Variables|Melting|SetMeltPoint _lerp)
      (Rendering|Material|SetScalarParameterValue (Variables|Default|GetCandleMaterial) "Anim" (Variables|Melting|GetMeltPoint) :!class /Script/Engine.MaterialInstanceDynamic)
      (if (== (Utilities|Array|Length (Variables|Default|GetFlames)) 1)
        (CallFunction|UpdateFlameLoc 0 (Variables|Melting|GetMeltPoint))
        (else
          (for (_ _array_index) (Variables|Default|GetFlames)
            (CallFunction|UpdateFlameLoc _array_index (Variables|Melting|GetMeltPoint))))))
    (:Finished
      (if (Variables|Melting|GetOffAfterMelt)
        (CallFunction|CandleOff true true)
        (Actor|DestroyActor)))))

(event EventCandleon
  ;[1 1 1] Start candle flame and melting
  (|CallParentFunction)
  (Components|Timeline|SetNewTime (Variables|Default|GetTimeline_Melting) (Variables|Melting|GetMeltPoint))
  ;[1 1 1] Handles melting animation, light and particle position
  (bind _lerp (Timeline|Timeline_Melting Play)
    (:Update
      (Variables|Melting|SetMeltPoint _lerp)
      (Rendering|Material|SetScalarParameterValue (Variables|Default|GetCandleMaterial) "Anim" (Variables|Melting|GetMeltPoint) :!class /Script/Engine.MaterialInstanceDynamic)
      (if (== (Utilities|Array|Length (Variables|Default|GetFlames)) 1)
        (CallFunction|UpdateFlameLoc 0 (Variables|Melting|GetMeltPoint))
        (else
          (for (_ _array_index) (Variables|Default|GetFlames)
            (CallFunction|UpdateFlameLoc _array_index (Variables|Melting|GetMeltPoint))))))
    (:Finished
      (if (Variables|Melting|GetOffAfterMelt)
        (CallFunction|CandleOff true true)
        (Actor|DestroyActor)))))

(event EventBeginPlay
  (for _array_element (Actor|GetAllChildActors false)
    (bind _asbp_lights_movable (Utilities|Casting|CastToBP_Lights_Movable _array_element))
    (Rendering|ToggleVisibility (Variables|/Game/MeltingCandlesPack/Blueprint/BP_Lights.BP_Lights_C|GetPointLight1 _asbp_lights_movable) true)
    (Rendering|ToggleVisibility (Variables|/Game/MeltingCandlesPack/Blueprint/BP_Lights.BP_Lights_C|GetPointLight _asbp_lights_movable) true)
    (Rendering|ToggleVisibility (Variables|/Game/MeltingCandlesPack/Blueprint/BP_Lights.BP_Lights_C|GetSpotLight _asbp_lights_movable) true)))

(fn ConstructionScript
  ;[1 1 1] variables on used in this child
  (Variables|Default|SetCandleState 0)
  (Variables|Default|SetRandomState false)
  (|CallParentFunction)
  ;[1 1 1] setups melt anim position in level
  (Rendering|Material|SetScalarParameterValue (Variables|Default|GetCandleMaterial) "Anim" (Variables|Melting|GetMeltPoint) :!class /Script/Engine.MaterialInstanceDynamic)
  (if (== (Utilities|Array|Length (Variables|Default|GetFlames)) 1)
    (CallFunction|UpdateFlameLoc 0 (Variables|Melting|GetMeltPoint))
    (else
      (for (_ _array_index) (Variables|Default|GetFlames)
        (CallFunction|UpdateFlameLoc _array_index (Variables|Melting|GetMeltPoint))))))

(fn SetupDynamicEffects
  (bind _returnvalue (Math|Random|RandomFloatinRange 0.3 1.0))
  ;[1 1 1] Add smoke mesh, particles and lights to selected mesh sockets. Construction script use only
  (Utilities|Map|Clear (Variables|Default|GetFlameStart/EndLoc))
  (for _array_element (Transformation|GetAllSocketNames (Variables|Default|GetSM_Candle))
    (if (Utilities|Enum|Equal(Enum) (Utilities|String|Left (Utilities|String|ToString(Name) _array_element) 9) "wick_str_")
      (LocalVariables|SetTampStartLoc (.location (Transformation|GetSocketTransform (Variables|Default|GetSM_Candle) _array_element "RTS_Actor")))
      (Utilities|FlowControl|Sequence
        (:then_0
          (bind _returnvalue_2 (AddComponent|AddParticleSystemComponent false (Math|Transform|MakeTransform (+ (LocalVariables|GetTampStartLoc) "0, 0,2.025042") "0, 0, 0" "1,1,1")))
          (Rendering|Material|SetMaterial _returnvalue_2 0 (Variables|Default|GetParticleMaterial))
          (Utilities|Array|Add (Variables|Default|GetFlames) _returnvalue_2)
          (LocalVariables|SetTempParticle _returnvalue_2))
        (:then_1
          (bind _returnvalue_3 (AddComponent|AddStaticMeshComponent false (Math|Transform|MakeTransform "0, 0,-2.025042" "0, 0, 0" (Math|Vector|MakeVector _returnvalue _returnvalue _returnvalue))))
          (Rendering|Material|SetMaterial _returnvalue_3 0 (Variables|Default|GetSmokeMat))
          (Transformation|AttachComponentToComponent _returnvalue_3 (LocalVariables|GetTempParticle) "None" "KeepRelative" "KeepRelative" "KeepWorld" true)
          (if (not (Variables|Default|GetNoLights))
            (bind _returnvalue_4 (AddComponent|AddChildActorComponent false (Math|Transform|MakeTransform (LocalVariables|GetTampStartLoc) "0, 0, 0" "1,1,1")))
            (ChildActorComponent|SetChildActorClass _returnvalue_4 (Utilities|Select :Index (Variables|Default|GetLightMobility) :NewEnumerator0 "/Game/MeltingCandlesPack/Blueprint/BP_Lights.BP_Lights_C" :NewEnumerator1 "/Game/MeltingCandlesPack/Blueprint/BP_Lights_stacionary.BP_Lights_stacionary_C" :NewEnumerator2 "/Game/MeltingCandlesPack/Blueprint/BP_Lights_Movable.BP_Lights_Movable_C"))
            (Transformation|AttachComponentToComponent _returnvalue_4 (LocalVariables|GetTempParticle) "None" "SnapToTarget" "KeepRelative" "KeepWorld" true))))
      (else
        (Utilities|Map|Add (Variables|Default|GetFlameStart/EndLoc) (LocalVariables|GetTampStartLoc) (.location (Transformation|GetSocketTransform (Variables|Default|GetSM_Candle) _array_element "RTS_Actor")))))))

(fn UpdateFlameLoc
  (params (Index :type Integer) (Alpha :type Float%20%28single-precision%29))
  ;[1 1 1] update particle location
  (bind _keys (Utilities|Map|Keys (Variables|Default|GetFlameStart/EndLoc)))
  (Transformation|SetRelativeLocation (Utilities|Array|Get(acopy) (Variables|Default|GetFlames) Index) (+ (Math|Vector|Lerp(Vector) (Utilities|Array|Get(acopy) _keys Index) (.Value (Utilities|Map|Find (Variables|Default|GetFlameStart/EndLoc) (Utilities|Array|Get(acopy) _keys Index))) Alpha) "0, 0,2.025042") false false))

(fn ConstructFunction
  ;[1 1 1] setups melt anim position in level
  (if (== (Utilities|Array|Length (Variables|Default|GetFlames)) 1)
    (CallFunction|UpdateFlameLoc 0 (Variables|Melting|GetMeltPoint))
    (else
      (for (_ _array_index) (Variables|Default|GetFlames)
        (CallFunction|UpdateFlameLoc _array_index (Variables|Melting|GetMeltPoint))))))