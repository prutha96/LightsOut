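; Child actor of BP_Candle that provides the candle's lighting through a point light and a spot light.
; Construction casts the parent actor to BP_Candle and copies its color, radius, shadow and intensity settings, zeroing both intensities when the flame is off.
; On BeginPlay, unless LightType is the first enum value, it binds the candle's dispatchers to update intensities, point-light shadows and shared color at runtime.
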(event Custom|EnentChangeIntencity
  (params (NewIntencity :type Float%20%28single-precision%29))
  ;[1 1 1] Binds event disbachers on begin play
  (Rendering|Components|Light|SetIntensity (Variables|Default|GetPointLight) NewIntencity))

(event Custom|EventChangeSS
  (params (NewIntensity :type Float%20%28single-precision%29))
  ;[1 1 1] Binds event disbachers on begin play
  (Rendering|Components|Light|SetIntensity (Variables|Default|GetSpotLight) NewIntensity))

(event Custom|ChangeLightShadows
  (params (On :type Boolean))
  ;[1 1 1] Binds event disbachers on begin play
  (Rendering|Components|Light|SetCastShadows (Variables|Default|GetPointLight) On))

(event Custom|EventChangeColor
  (params (NewColor :type Linear%20Color%20Structure))
  ;[1 1 1] Binds event disbachers on begin play
  (Rendering|Components|Light|SetLightColor (Variables|Default|GetSpotLight) NewColor true))

(event EventBeginPlay
  ;[1 1 1] Binds event disbachers on begin play
  (if (Utilities|Enum|NotEqual(Enum) (Variables|Default|GetLightType) "NewEnumerator0")
    (EventDispatchers|AssignChangeLightIntensity (Variables|Default|GetOwningCandle) (delegate Custom|EnentChangeIntencity))
    (EventDispatchers|AssignChangeLightSS (Variables|Default|GetOwningCandle) (delegate Custom|EventChangeSS))
    (EventDispatchers|AssignChangeLightShadows (Variables|Default|GetOwningCandle) (delegate Custom|ChangeLightShadows))
    (EventDispatchers|AssignChangeLightColor (Variables|Default|GetOwningCandle) (delegate Custom|EventChangeColor))))

(fn ConstructionScript
  ;[1 1 1] get light data from candle parent
  (bind _asbp_candle (Utilities|Casting|CastToBP_Candle (Actor|GetParentActor)))
  (bind _output_get (Variables|Default|SetOwningCandle _asbp_candle))
  (if (Variables|/Game/MeltingCandlesPack/Blueprint/BP_Candle.BP_Candle_C|GetCandleFlameOn _output_get)
    (Rendering|Components|Light|SetIntensity (Variables|Default|GetPointLight) (Variables|/Game/MeltingCandlesPack/Blueprint/BP_Candle.BP_Candle_C|GetLightIntencity (Variables|Default|GetOwningCandle)))
    (Rendering|Lighting|SetAttenuationRadius (Variables|Default|GetPointLight) (Variables|/Game/MeltingCandlesPack/Blueprint/BP_Candle.BP_Candle_C|GetAttenuationRadius (Variables|Default|GetOwningCandle)))
    (Rendering|Components|Light|SetCastShadows (Variables|Default|GetPointLight) (Variables|/Game/MeltingCandlesPack/Blueprint/BP_Candle.BP_Candle_C|GetLightShadows (Variables|Default|GetOwningCandle)))
    (Rendering|Components|Light|SetLightColor (Variables|Default|GetPointLight) (Variables|/Game/MeltingCandlesPack/Blueprint/BP_Candle.BP_Candle_C|GetFlameColor (Variables|Default|GetOwningCandle)) true)
    (Rendering|Components|Light|SetLightColor (Variables|Default|GetSpotLight) (Variables|/Game/MeltingCandlesPack/Blueprint/BP_Candle.BP_Candle_C|GetFlameColor (Variables|Default|GetOwningCandle)) true)
    (Rendering|Components|Light|SetIntensity (Variables|Default|GetSpotLight) (Variables|/Game/MeltingCandlesPack/Blueprint/BP_Candle.BP_Candle_C|GetSSLight (Variables|Default|GetOwningCandle)))
    (else
      (Rendering|Components|Light|SetIntensity (Variables|Default|GetPointLight) 0.0)
      (Rendering|Lighting|SetAttenuationRadius (Variables|Default|GetPointLight) (Variables|/Game/MeltingCandlesPack/Blueprint/BP_Candle.BP_Candle_C|GetAttenuationRadius (Variables|Default|GetOwningCandle)))
      (Rendering|Components|Light|SetCastShadows (Variables|Default|GetPointLight) (Variables|/Game/MeltingCandlesPack/Blueprint/BP_Candle.BP_Candle_C|GetLightShadows (Variables|Default|GetOwningCandle)))
      (Rendering|Components|Light|SetLightColor (Variables|Default|GetPointLight) (Variables|/Game/MeltingCandlesPack/Blueprint/BP_Candle.BP_Candle_C|GetFlameColor (Variables|Default|GetOwningCandle)) true)
      (Rendering|Components|Light|SetLightColor (Variables|Default|GetSpotLight) (Variables|/Game/MeltingCandlesPack/Blueprint/BP_Candle.BP_Candle_C|GetFlameColor (Variables|Default|GetOwningCandle)) true)
      (Rendering|Components|Light|SetIntensity (Variables|Default|GetSpotLight) 0.0))))